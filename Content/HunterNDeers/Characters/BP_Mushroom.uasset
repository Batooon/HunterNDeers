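; BP_Mushroom is a mushroom pickup in Hunter N Deers that shows an interaction prompt to deer players.
; A sphere overlap shows the MushroomInteraction component for a locally controlled BP_Deer that is not eating, and hides it when that deer leaves.
; While visible, the shadowless prompt rotates each tick to face the local camera, acting as a billboard.
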(event `self.ReceiveBeginPlay`
  (`PrimitiveComponent.SetCastShadow` (`self.MushroomInteraction`) false)
  (`self.TogglePlayerInteraction` false))

(event `self.ReceiveTick`
  (params (DeltaSeconds :type "Float (single-precision)"))
  (if (`self.bPlayerInTriggerDistance`)
    (`SceneComponent.K2_SetWorldRotation` (`self.MushroomInteraction`) (`KismetMathLibrary.FindLookAtRotation` (`SceneComponent.K2_GetComponentLocation` (`self.MushroomInteraction`)) (`SceneComponent.K2_GetComponentLocation` (`PlayerCameraManager.TransformComponent` (`GameplayStatics.GetPlayerCameraManager` 0)))) false false)))

(event `self.Sphere.OnComponentBeginOverlap`
  (params (OverlappedComponent :type "PrimitiveComponent Object Reference") (OtherActor :type "Actor Object Reference") (OtherComp :type "PrimitiveComponent Object Reference") (OtherBodyIndex :type Integer) (bFromSweep :type Boolean) (SweepResult :type "HitResult Structure (by ref)"))
  (bind _asbp_deer (cast `/Game/HunterNDeers/Characters/BP_Deer` OtherActor))
  (if (and (`Pawn.IsLocallyControlled` _asbp_deer) (not (`/Game/HunterNDeers/Characters/BP_Deer.bEating` _asbp_deer)))
    (`self.TogglePlayerInteraction` true)))

(event `self.Sphere.OnComponentEndOverlap`
  (params (OverlappedComponent :type "PrimitiveComponent Object Reference") (OtherActor :type "Actor Object Reference") (OtherComp :type "PrimitiveComponent Object Reference") (OtherBodyIndex :type Integer))
  (bind _asbp_deer (cast `/Game/HunterNDeers/Characters/BP_Deer` OtherActor))
  (if (and (`Pawn.IsLocallyControlled` _asbp_deer) (`self.bPlayerInTriggerDistance`))
    (`self.TogglePlayerInteraction` false)))

(fn `TogglePlayerInteraction`
  (params (bPlayerInTriggerDistance :type Boolean))
  (bind _output_get (set `self.bPlayerInTriggerDistance` bPlayerInTriggerDistance))
  (`SceneComponent.SetVisibility` (`self.MushroomInteraction`) _output_get false))

(fn `UserConstructionScript`)