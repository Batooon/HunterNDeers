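; BP_AIDeer is the AI-controlled deer character in the HunterNDeers game, a prey NPC that grazes and can be killed by arrows.
; Eat and StopEating play and blend out a doe idle-graze montage on the mesh's anim instance, cached at BeginPlay.
; HitbyArrow reports the kill to BP_GameState through OnNPCDeerKilled, then destroys the actor.
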(event `self.ReceiveBeginPlay`
  (set `self.MeshAnim` (`SkeletalMeshComponent.GetAnimInstance` (`self.Mesh`))))

(event `Eat`
  (`AnimInstance.Montage_Play` (`self.MeshAnim`) "/Game/HunterNDeers/Characters/DeerStagAndDoe/Animations/ANIM_DeerDoe_IdleGraze_Montage.ANIM_DeerDoe_IdleGraze_Montage" 1.0 "MontageLength" 0.0 false))

(event `StopEating`
  (`AnimInstance.Montage_Stop` (`self.MeshAnim`) 0.25 "/Game/HunterNDeers/Characters/DeerStagAndDoe/Animations/ANIM_DeerDoe_IdleGraze_Montage.ANIM_DeerDoe_IdleGraze_Montage"))

(event `/Game/HunterNDeers/Characters/BPI_ArrowHittable.HitByArrow`
  (`/Game/HunterNDeers/Core/BP_GameState.OnNPCDeerKilled` (cast `/Game/HunterNDeers/Core/BP_GameState` (`GameplayStatics.GetGameState`) :!pure true))
  (`self.K2_DestroyActor`))

(fn `UserConstructionScript`)