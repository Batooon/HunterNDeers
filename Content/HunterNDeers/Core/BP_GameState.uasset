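; Game state for HunterNDeers that starts a match once enough players connect and picks the hunter.
; Connection updates refresh the player count and, upon reaching the game mode's minimum, trigger a one-time countdown on a one-second delay loop.
; At zero, a randomly indexed player controller transforms into the hunter and game start is broadcast.
; RepNotify functions relay player count and countdown changes through event dispatchers.
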(event `PlayerConnectionUpdated`
  (bind _returnvalue (`GameplayStatics.GetNumPlayerStates`))
  (set `self.PlayersAmount` _returnvalue)
  (if (>= _returnvalue (`/Game/FirstPerson/Blueprints/BP_FirstPersonGameMode.MinimumRequiredPlayers` (cast `/Game/FirstPerson/Blueprints/BP_FirstPersonGameMode` (`GameplayStatics.GetGameMode`) :!pure true)))
    (`/Engine/EditorBlueprintResources/StandardMacros.DoOnce` false
      (:`Completed`
        (`self.StartGameCountdown`)))))

(event `StartGameCountdown`
  (set `self.CurrentGameCountdownTime` (`self.StartGameCountdownTime`))
  (if (> (`self.CurrentGameCountdownTime`) 0) :!label _label
    (set `self.CurrentGameCountdownTime` (- (`self.CurrentGameCountdownTime`) 1))
    (`KismetSystemLibrary.Delay` 1.0)
    (goto _label)
    (else
      (`/Game/FirstPerson/Blueprints/BP_FirstPersonPlayerController.TransformToHunter` (cast `/Game/FirstPerson/Blueprints/BP_FirstPersonPlayerController` (`GameplayStatics.GetPlayerController` (`KismetMathLibrary.RandomInteger` (`self.PlayersAmount`))) :!pure true))
      (`self.StartGame`))))

(event `StartGame`
  (`self.GameStarted`))

(fn `OnRep_CurrentGameCountdownTime`
  (`self.GameCountdownUpdated` (`self.CurrentGameCountdownTime`)))

(fn `OnRep_PlayersAmount`
  (`self.PlayersAmountChanged` (`self.PlayersAmount`)))

(fn `UserConstructionScript`)