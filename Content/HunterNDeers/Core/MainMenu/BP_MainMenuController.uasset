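; BP_MainMenuController is the player controller for the main menu, showing the menu and handling session hosting and joining.
; On BeginPlay it creates WBP_MainMenu and adds it to the viewport for the local player only.
; Create&JoinNewSession starts a five-slot, non-LAN session and, on success, opens the Forest level with the passed options.
; JoinSession joins a supplied search result.
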(event `self.ReceiveBeginPlay`
  (if (`self.IsLocalPlayerController`)
    (bind _returnvalue (`|CreateWidget` "/Game/HunterNDeers/Widgets/WBP_MainMenu.WBP_MainMenu_C"))
    (`UserWidget.AddToViewport` _returnvalue 0)))

(event `Create&JoinNewSession`
  (params (Options :type String))
  (`CreateSessionCallbackProxy.CreateSession` self 5
    (:`OnSuccess`
      (`GameplayStatics.OpenLevelBySoftObjectPtr` "/Game/HunterNDeers/Maps/Forest.Forest" true Options))))

(event `JoinSession`
  (params (Session :type "BlueprintSessionResult Structure"))
  (`JoinSessionCallbackProxy.JoinSession` self Session))

(fn `UserConstructionScript`)